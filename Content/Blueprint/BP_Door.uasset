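; Colour-coded door actor that swings open when the player has collected at least three of the matching Red, Green or Blue.
; BeginPlay caches BP_Richard and computes an open rotation at -120 degrees yaw from the mesh's start.
; Box overlap by a Player-tagged actor matches the door's own tags to that count, then plays a shared Timeline lerping from current rotation toward open.
; The Open function is empty.
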(event `self.ReceiveBeginPlay`
  (bind (_returnvalue_roll _returnvalue_pitch _returnvalue_yaw) (`KismetMathLibrary.BreakRotator` (`SceneComponent.K2_GetComponentRotation` (`self.StaticMesh`))))
  (`|ExecutionSequence`
    (:`then_0`
      (set `self.OpenRotation` (`KismetMathLibrary.MakeRotator` _returnvalue_roll _returnvalue_pitch (+ _returnvalue_yaw -120.0))))
    (:`then_1`
      (bind _asbp_richard (cast `/Game/Blueprint/BP_Richard` (`GameplayStatics.GetPlayerCharacter` 0)))
      (set `self.Player` _asbp_richard))))

(event `self.Box.OnComponentBeginOverlap`
  (params (OverlappedComponent :type "PrimitiveComponent Object Reference") (OtherActor :type "Actor Object Reference") (OtherComp :type "PrimitiveComponent Object Reference") (OtherBodyIndex :type Integer) (bFromSweep :type Boolean) (SweepResult :type "HitResult Structure (by ref)"))
  (bind _player (`self.Player`))
  (bind _reds (`/Game/Blueprint/BP_Richard.Reds` _player))
  (if (`self.ActorHasTag` OtherActor "Player")
    (for _array_element (`self.Tags`)
      (`|ExecutionSequence`
        (:`then_0`
          (if (== _array_element "Red")
            (`KismetSystemLibrary.PrintString` (`KismetStringLibrary.Conv_IntToString` _reds))
            (if (>= _reds 3)
              (bind (_direction _newtrack_0) (`Timeline|Timeline` :!label _label)
                (:`Update`
                  (`SceneComponent.K2_SetWorldRotation` (`self.StaticMesh`) (`KismetMathLibrary.RLerp` (`SceneComponent.K2_GetComponentRotation` (`self.StaticMesh`)) (`self.OpenRotation`) _newtrack_0) false false))))))
        (:`then_1`
          (if (== _array_element "Green")
            (if (>= (`/Game/Blueprint/BP_Richard.Greens` _player) 3)
              (goto _label))))
        (:`then_2`
          (if (== _array_element "Blue")
            (if (>= (`/Game/Blueprint/BP_Richard.Blues` _player) 3)
              (goto _label))))))))

(fn `Open`)

(fn `UserConstructionScript`)