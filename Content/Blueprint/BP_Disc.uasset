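; BP_Disc is a colour-tagged disc that, when hit, swaps its cylinder's material and can turn on a linked light.
; It caches the BP_Richard player on BeginPlay, then on each Hit loops over its own Tags for Red, Green or Blue.
; A matching tag turns on the Light only if the player's counter for that colour equals three, with a debug print on the red branch.
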(event `self.ReceiveBeginPlay`
  (bind _asbp_richard (cast `/Game/Blueprint/BP_Richard` (`GameplayStatics.GetPlayerCharacter` 0)))
  (set `self.Player` _asbp_richard))

(event `self.ReceiveHit`
  (params (MyComp :type "PrimitiveComponent Object Reference") (Other :type "Actor Object Reference") (OtherComp :type "PrimitiveComponent Object Reference") (bSelfMoved :type Boolean) (HitLocation :type "Vector Structure") (HitNormal :type "Vector Structure") (NormalImpulse :type "Vector Structure") (Hit :type "HitResult Structure (by ref)"))
  (bind _player (`self.Player`))
  (bind _reds (`/Game/Blueprint/BP_Richard.Reds` _player))
  (`PrimitiveComponent.SetMaterial` (`self.Cylinder`) 0 (`self.Material`))
  (for _array_element (`self.Tags`)
    (`|ExecutionSequence`
      (:`then_0`
        (if (== _array_element "Red")
          (if (== _reds 3)
            (`/Game/Blueprint/BP_DoorLight.TurnOnLight` (`self.Light`))
            (`KismetSystemLibrary.PrintString` (`KismetStringLibrary.Conv_IntToString` _reds)))))
      (:`then_1`
        (if (== _array_element "Green")
          (if (== (`/Game/Blueprint/BP_Richard.Greens` _player) 3)
            (`/Game/Blueprint/BP_DoorLight.TurnOnLight` (`self.Light`)))))
      (:`then_2`
        (if (== _array_element "Blue")
          (if (== (`/Game/Blueprint/BP_Richard.Blues` _player) 3)
            (`/Game/Blueprint/BP_DoorLight.TurnOnLight` (`self.Light`))))))))

(fn `UserConstructionScript`)